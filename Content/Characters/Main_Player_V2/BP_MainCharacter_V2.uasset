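; Player character that walks under custom gravity and throws snowballs.
; Tick points CharacterMovement gravity at MTargetGravityActor when valid, allowing planet-style gravity.
; IA_Move converts control rotation into gravity-relative space, drops pitch, then converts back to get movement directions.
; Left mouse plays AM_Throw behind a DoOnce that resets on completion, spawning the projectile at ProjectileStartLoc on the montage notify.
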(event Input|EnhancedActionEvents|EnhancedInputActionIA_Move
  (params (ActionValue :type Vector%202D%20Structure) (ElapsedSeconds :type Float%20%28double-precision%29) (TriggeredSeconds :type Float%20%28double-precision%29) (InputAction :type Input%20Action%20Object%20Reference :default "/Game/ThirdPerson/Input/Actions/IA_Move.IA_Move"))
  (bind _returnvalue (Pawn|GetControlRotation :!class /Script/Engine.Pawn))
  (bind _returnvalue_2 (Pawn|GetControlRotation :!class /Script/Engine.Pawn))
  (bind _charactermovement (Variables|Character|GetCharacterMovement))
  (bind _charactermovement_2 (Variables|Character|GetCharacterMovement))
  (bind _gravitydirection (Variables|/Script/Engine.CharacterMovementComponent|GetGravityDirection _charactermovement_2))
  (bind _gravitydirection_2 (Variables|/Script/Engine.CharacterMovementComponent|GetGravityDirection _charactermovement))
  (bind _returnvalue_3 (Class|GravityController|GetGravityRelativeRotation _returnvalue_2 _gravitydirection))
  (bind _returnvalue_4 (Class|GravityController|GetGravityRelativeRotation _returnvalue _gravitydirection_2))
  ;[0 0.03906 1] Move
  (Pawn|Input|AddMovementInput (Math|Vector|GetRightVector (Class|GravityController|GetGravityWorldRotation (Math|Rotator|MakeRotator (.roll _returnvalue_3) 0.0 (.yaw _returnvalue_3)) _gravitydirection)) (.x ActionValue) false)
  (Pawn|Input|AddMovementInput (Math|Vector|GetForwardVector (Class|GravityController|GetGravityWorldRotation (Math|Rotator|MakeRotator (.roll _returnvalue_4) 0.0 (.yaw _returnvalue_4)) _gravitydirection_2)) (.y ActionValue) false))

(event EventBeginPlay)

(event Collision|EventActorBeginOverlap
  (params (OtherActor :type Actor%20Object%20Reference)))

(event EventTick
  (params (DeltaSeconds :type Float%20%28single-precision%29))
  (bind _m_targetgravityactor (Variables|Default|Getm_TargetGravityActor))
  ;[1 0.8906 0] Comment
  ;;[1 0.3984 0] Set Gravity On Tick
  (Utilities|IsValid _m_targetgravityactor
    (:Is%20Valid
      (Class|CharacterMovementComponent|SetGravityDirection (Variables|Character|GetCharacterMovement) (Math|Vector|Normalize (- (Transformation|GetActorLocation _m_targetgravityactor) (Transformation|GetActorLocation)))))))

(event Input|MouseEvents|LeftMouseButton
  (params (Key :type Key%20Structure :default "None"))
  (bind _projectilestartloc (Variables|Default|GetProjectileStartLoc))
  ;[0 1 0.6719] Comment
  (:Pressed
    (Utilities|FlowControl|DoOnce false :!label _label
      (:Completed
        (bind _notifyname (Animation|Montage|PlayMontage (Variables|Character|GetMesh) "/Game/Characters/Main_Player/Animations/AM_Throw.AM_Throw")
          (:OnCompleted
            (goto _label Reset))
          (:OnNotifyBegin
            (switch name _notifyname
              (:Throw
                (Game|SpawnActorfromClass "/Game/TinySnowWorld/Blueprints/SnowBallProjectile_BP.SnowBallProjectile_BP_C" (Math|Transform|MakeTransform (Transformation|GetWorldLocation _projectilestartloc) (Transformation|GetWorldRotation _projectilestartloc) "1.000000,1.000000,1.000000") "Undefined" "MultiplyWithRoot" self 0)))))))))

(fn ConstructionScript)