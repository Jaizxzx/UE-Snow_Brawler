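; BP_Enemy_Master is an enemy character that detects the player and throws snowballs.
; Perception updates set or clear the Enemy on its cached BP_AiC_Enemy controller when it senses or loses BP_Main_Player_Grav.
; A Focus event sets or clears controller focus on that enemy.
; Shoot plays a throw montage behind a DoOnce that resets on completion, spawning SnowBallProjectile_BP ahead of the enemy at the montage notify.
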(event OnTargetPerceptionUpdated(AIPerception)
  (params (Actor :type Actor%20Object%20Reference) (Stimulus :type AI%20Stimulus%20Structure))
  ;[1 0.07031 0] Update Sight
  (bind _asbp_main_player_grav (Utilities|Casting|CastToBP_Main_Player_Grav Actor))
  (bind _aicont_ref (Variables|References|GetAiCont%20Ref)
    (:then
      (if (Utilities|Struct|BreakAIStimulus Stimulus)
        (Default|SetEnemy _aicont_ref _asbp_main_player_grav)
        (else
          (Default|SetEnemy _aicont_ref))))
    (:else)))

(event EventBeginPlay
  ;[0 1 0.9063] Get Aic Ref
  (bind _asbp_ai_c_enemy (Utilities|Casting|CastToBP_AiC_Enemy (AI|GetAIController self)))
  (Variables|References|SetAiCont%20Ref _asbp_ai_c_enemy))

(event EventShoot
  (bind _returnvalue (Transformation|GetActorTransform))
  (bind _self self)
  ;[1 0 0.07031] Shoot
  (Utilities|FlowControl|DoOnce false :!label _label
    (:Completed
      (bind _notifyname (Animation|Montage|PlayMontage (Variables|Character|GetMesh) "/Game/Characters/Main_Player/Animations/AM_Throw.AM_Throw")
        (:OnCompleted
          (goto _label Reset))
        (:OnNotifyBegin
          (switch name _notifyname
            (:Throw
              (Game|SpawnActorfromClass "/Game/TinySnowWorld/Blueprints/SnowBallProjectile_BP.SnowBallProjectile_BP_C" (Math|Transform|MakeTransform (+ (.location _returnvalue) (* (Transformation|GetActorForwardVector) 1.5e+02)) (.rotation _returnvalue) (.scale _returnvalue)) "Undefined" "MultiplyWithRoot" _self _self))))))))

(event EventFocus
  (params (Focus? :type Boolean))
  ;[0 1 0.08594] Focus Update
  (bind _aicont_ref (Variables|References|GetAiCont%20Ref)
    (:then
      (if Focus?
        (AI|SetFocus _aicont_ref (Variables|/Game/Blueprints/Ai/BP_AiC_Enemy.BP_AiC_Enemy_C|GetEnemy _aicont_ref))
        (else
          (AI|ClearFocus _aicont_ref))))
    (:else)))

(fn ConstructionScript)