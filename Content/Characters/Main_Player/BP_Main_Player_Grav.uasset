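; Player character that walks under custom gravity and throws snowballs.
; Each tick, gravity is pointed toward MTargetGravityActor when valid, and movement input converts control rotation into gravity-relative directions.
; Left mouse plays a throw montage that spawns the snowball projectile at the actor transform on notify, with a DoOnce blocking repeats until completion.
; Enhanced Input drives look and move, while jump is disabled.
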(event Input|EnhancedActionEvents|EnhancedInputActionIA_Look
  (params (ActionValue :type Vector%202D%20Structure) (ElapsedSeconds :type Float%20%28double-precision%29) (TriggeredSeconds :type Float%20%28double-precision%29) (InputAction :type Input%20Action%20Object%20Reference :default "/Game/ThirdPerson/Input/Actions/IA_Look.IA_Look"))
  ;[0 0.5312 1] Look
  (Pawn|Input|AddControllerYawInput (.x ActionValue))
  (Pawn|Input|AddControllerPitchInput (.y ActionValue)))

(event Input|EnhancedActionEvents|EnhancedInputActionIA_Move
  (params (ActionValue :type Vector%202D%20Structure) (ElapsedSeconds :type Float%20%28double-precision%29) (TriggeredSeconds :type Float%20%28double-precision%29) (InputAction :type Input%20Action%20Object%20Reference :default "/Game/ThirdPerson/Input/Actions/IA_Move.IA_Move"))
  (bind _returnvalue (Pawn|GetControlRotation :!class /Script/Engine.Pawn))
  (bind _returnvalue_2 (Pawn|GetControlRotation :!class /Script/Engine.Pawn))
  (bind _charactermovement (Variables|Character|GetCharacterMovement))
  (bind _charactermovement_2 (Variables|Character|GetCharacterMovement))
  (bind _gravitydirection (Variables|/Script/Engine.CharacterMovementComponent|GetGravityDirection _charactermovement))
  (bind _gravitydirection_2 (Variables|/Script/Engine.CharacterMovementComponent|GetGravityDirection _charactermovement_2))
  (bind _returnvalue_3 (Class|GravityController|GetGravityRelativeRotation _returnvalue_2 _gravitydirection_2))
  (bind _returnvalue_4 (Class|GravityController|GetGravityRelativeRotation _returnvalue _gravitydirection))
  ;[0 0.03906 1] Move
  (Pawn|Input|AddMovementInput (Math|Vector|GetRightVector (Class|GravityController|GetGravityWorldRotation (Math|Rotator|MakeRotator (.roll _returnvalue_3) 0.0 (.yaw _returnvalue_3)) _gravitydirection_2)) (.x ActionValue) false)
  (Pawn|Input|AddMovementInput (Math|Vector|GetForwardVector (Class|GravityController|GetGravityWorldRotation (Math|Rotator|MakeRotator (.roll _returnvalue_4) 0.0 (.yaw _returnvalue_4)) _gravitydirection)) (.y ActionValue) false))

(event Input|EnhancedActionEvents|EnhancedInputActionIA_Jump
  (params (ActionValue :type Boolean) (ElapsedSeconds :type Float%20%28double-precision%29) (TriggeredSeconds :type Float%20%28double-precision%29) (InputAction :type Input%20Action%20Object%20Reference :default "/Game/ThirdPerson/Input/Actions/IA_Jump.IA_Jump"))
  ;[0.3125 1 0] Jump ( Disabled for now ) !!!!
)

(event EventBeginPlay
  (bind _returnvalue (Game|GetPlayerController 0))
  (bind _returnvalue_2 (PlayerController|LocalPlayerSubsystems|GetEnhancedInputLocalPlayerSubsystem _returnvalue))
  ;[1 0.7266 0] Input Context Mapping
  (Utilities|IsValid _returnvalue_2
    (:Is%20Valid
      (Input|AddMappingContext _returnvalue_2 "/Game/ThirdPerson/Input/IMC_Default.IMC_Default" 0 "(bIgnoreAllPressedKeysUntilRelease=True,bForceImmediately=False,bNotifyUserSettings=False)"))))

(event EventTick
  (params (DeltaSeconds :type Float%20%28single-precision%29))
  (bind _m_targetgravityactor (Variables|Default|Getm_TargetGravityActor))
  ;[0 1 0.8125] SetGravityOnTick
  (Utilities|IsValid _m_targetgravityactor
    (:Is%20Valid
      (Class|CharacterMovementComponent|SetGravityDirection (Variables|Character|GetCharacterMovement) (Math|Vector|Normalize (- (Transformation|GetActorLocation _m_targetgravityactor) (Transformation|GetActorLocation)))))))

(event Input|MouseEvents|LeftMouseButton
  (params (Key :type Key%20Structure :default "None"))
  (bind _self self)
  ;[1 0 0.375] Throw logic
  (:Pressed
    (Utilities|FlowControl|DoOnce false :!label _label
      (:Completed
        (bind _notifyname (Animation|Montage|PlayMontage (Variables|Character|GetMesh) "/Game/Characters/Main_Player/Animations/AM_Throw.AM_Throw")
          (:OnCompleted
            (goto _label Reset))
          (:OnNotifyBegin
            (switch name _notifyname
              (:Throw
                (Game|SpawnActorfromClass "/Game/TinySnowWorld/Blueprints/SnowBallProjectile_BP.SnowBallProjectile_BP_C" (Transformation|GetActorTransform) "Undefined" "MultiplyWithRoot" _self _self)))))))))

(fn ConstructionScript)