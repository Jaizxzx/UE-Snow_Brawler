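; Gravity zone actor that uses a sphere trigger to switch which gravity actor a TiCharacter targets.
; Entering characters receive the on-overlap target and exiting ones the end-overlap target.
; Other entering actors go to AddActorToMap, but exit does not remove them because the RemoveActorFromMap call is unwired.
; A Blueprint radial force calculation for physics bodies is also disconnected, and Tick is empty.
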(event OnComponentBeginOverlap(Sphere)
  (params (OverlappedComponent :type Primitive%20Component%20Object%20Reference) (OtherActor :type Actor%20Object%20Reference) (OtherComp :type Primitive%20Component%20Object%20Reference) (OtherBodyIndex :type Integer) (bFromSweep :type Boolean) (SweepResult :type Hit%20Result%20Structure%20%28by%20ref%29))
  (bind _asti_character (Utilities|Casting|CastToTiCharacter OtherActor)
    (:then
      (Variables|/Script/WTF.TiCharacter|Setm_TargetGravityActor _asti_character (Variables|Default|Getm_OnTargetGravityActor)))
    (:CastFailed
      (Class|GravityAffector|AddActortoMap OtherActor))))

(event OnComponentEndOverlap(Sphere)
  (params (OverlappedComponent :type Primitive%20Component%20Object%20Reference) (OtherActor :type Actor%20Object%20Reference) (OtherComp :type Primitive%20Component%20Object%20Reference) (OtherBodyIndex :type Integer))
  (bind _asti_character (Utilities|Casting|CastToTiCharacter OtherActor))
  (Variables|/Script/WTF.TiCharacter|Setm_TargetGravityActor _asti_character (Variables|Default|Getm_EndTargetGravityActor)))

(event EventBeginPlay)

(event Collision|EventActorBeginOverlap
  (params (OtherActor :type Actor%20Object%20Reference)))

(event EventTick
  (params (DeltaSeconds :type Float%20%28single-precision%29)))

(fn ConstructionScript)