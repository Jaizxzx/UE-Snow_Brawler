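; Test player character for a snowball-throwing game that walks under custom gravity pointing toward a target actor, as on a small planet.
; Tick aims CharacterMovement gravity at that actor, and Enhanced Input move converts control rotation through gravity-relative space.
; Left mouse plays a throw montage behind a one-second gate, while a separate left-mouse handler spawns a snowball projectile ungated.
; Jump is disabled.
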(event Input|EnhancedActionEvents|EnhancedInputActionIA_Look
  (params (ActionValue :type Vector%202D%20Structure) (ElapsedSeconds :type Float%20%28double-precision%29) (TriggeredSeconds :type Float%20%28double-precision%29) (InputAction :type Input%20Action%20Object%20Reference :default "/Game/ThirdPerson/Input/Actions/IA_Look.IA_Look"))
  ;[0 0.5312 1] Look
  (Pawn|Input|AddControllerYawInput (.x ActionValue))
  (Pawn|Input|AddControllerPitchInput (.y ActionValue)))

(event Input|EnhancedActionEvents|EnhancedInputActionIA_Move
  (params (ActionValue :type Vector%202D%20Structure) (ElapsedSeconds :type Float%20%28double-precision%29) (TriggeredSeconds :type Float%20%28double-precision%29) (InputAction :type Input%20Action%20Object%20Reference :default "/Game/ThirdPerson/Input/Actions/IA_Move.IA_Move"))
  (bind _returnvalue (Pawn|GetControlRotation :!class /Script/Engine.Pawn))
  (bind _returnvalue_2 (Pawn|GetControlRotation :!class /Script/Engine.Pawn))
  (bind _charactermovement (Variables|Character|GetCharacterMovement))
  (bind _charactermovement_2 (Variables|Character|GetCharacterMovement))
  (bind _gravitydirection (Variables|/Script/Engine.CharacterMovementComponent|GetGravityDirection _charactermovement))
  (bind _gravitydirection_2 (Variables|/Script/Engine.CharacterMovementComponent|GetGravityDirection _charactermovement_2))
  (bind _returnvalue_3 (Class|GravityController|GetGravityRelativeRotation _returnvalue_2 _gravitydirection_2))
  (bind _returnvalue_4 (Class|GravityController|GetGravityRelativeRotation _returnvalue _gravitydirection))
  (Pawn|Input|AddMovementInput (Math|Vector|GetRightVector (Class|GravityController|GetGravityWorldRotation (Math|Rotator|MakeRotator (.roll _returnvalue_3) 0.0 (.yaw _returnvalue_3)) _gravitydirection_2)) (.x ActionValue) false)
  (Pawn|Input|AddMovementInput (Math|Vector|GetForwardVector (Class|GravityController|GetGravityWorldRotation (Math|Rotator|MakeRotator (.roll _returnvalue_4) 0.0 (.yaw _returnvalue_4)) _gravitydirection)) (.y ActionValue) false))

(event Input|EnhancedActionEvents|EnhancedInputActionIA_Jump
  (params (ActionValue :type Boolean) (ElapsedSeconds :type Float%20%28double-precision%29) (TriggeredSeconds :type Float%20%28double-precision%29) (InputAction :type Input%20Action%20Object%20Reference :default "/Game/ThirdPerson/Input/Actions/IA_Jump.IA_Jump"))
  ;[0.3125 1 0] Jump ( Disabled for now ) !!!!
)

(event EventBeginPlay
  ;[1 0.7266 0] Input Context Mapping
  (bind _asmain_player_controller (Utilities|Casting|CastToMain_PlayerController (Game|GetPlayerController 0)))
  (Utilities|IsValid (PlayerController|LocalPlayerSubsystems|GetEnhancedInputLocalPlayerSubsystem _asmain_player_controller)
    (:Is%20Valid
      (Input|AddMappingContext (PlayerController|LocalPlayerSubsystems|GetEnhancedInputLocalPlayerSubsystem _asmain_player_controller) "/Game/ThirdPerson/Input/IMC_Default.IMC_Default" 0 "(bIgnoreAllPressedKeysUntilRelease=True,bForceImmediately=False,bNotifyUserSettings=False)"))))

(event EventTick
  (params (DeltaSeconds :type Float%20%28single-precision%29))
  (Utilities|IsValid 0
    (:Is%20Valid
      (Class|CharacterMovementComponent|SetGravityDirection (Variables|Character|GetCharacterMovement) (Math|Vector|Normalize (- (Transformation|GetActorLocation (Variables|Default|Getm_TargetGravityActor)) (Transformation|GetActorLocation)))))))

(event Input|MouseEvents|LeftMouseButton
  (params (Key :type Key%20Structure :default "None"))
  (bind _projectilestartloc (Variables|Default|GetProjectileStartLoc))
  (:Pressed
    (Game|SpawnActorfromClass "/Game/TinySnowWorld/Blueprints/SnowBallProjectile_BP.SnowBallProjectile_BP_C" (Math|Transform|MakeTransform (Transformation|GetWorldLocation _projectilestartloc) (Transformation|GetWorldRotation _projectilestartloc) "1.000000,1.000000,1.000000") "Undefined" "MultiplyWithRoot" 0 0)))

(event Input|MouseEvents|LeftMouseButton
  (params (Key :type Key%20Structure :default "None"))
  ;[1 0 0.375] Throw logic
  (:Pressed
    (Utilities|FlowControl|DoOnce false :!label _label
      (:Completed
        (Animation|PlayAnimMontage "/Game/Characters/Main_Player/Animations/AM_Throw.AM_Throw" 1.0 "None")
        (Utilities|FlowControl|Delay 1.0)
        (goto _label Reset)))))

(fn ConstructionScript)